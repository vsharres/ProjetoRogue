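; Room Blueprint (Sala_1P_BP2) for an enemy encounter with locking doors and a HUD enemy health bar.
; On BeginPlay it collects Porta_Normal child actors as its doors and sets itself as their parent room.
; Trigger overlaps go to activation handlers; AtualizarVidaInimigos locks the doors, passes the enemies to the player's HUD and unbinds the trigger.
; DestrancarPortas hides the enemy health display and recolors the room green.
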(event OnComponentBeginOverlap(TriggerAtivarInimigos)
  (params (OtherActor :type Actor%20Object%20Reference) (OtherComp :type Primitive%20Component%20Object%20Reference) (OtherBodyIndex :type Integer) (bFromSweep :type Boolean) (SweepResult :type Hit%20Result%20Structure%20%28by%20ref%29))
  (Class|Sala|AtivarInimigosTriggeronOverlap OtherActor))

(event OnComponentEndOverlap(TriggerAtivarInimigos)
  (params (OtherActor :type Actor%20Object%20Reference) (OtherComp :type Primitive%20Component%20Object%20Reference) (OtherBodyIndex :type Integer))
  (Class|Sala|AtivarInimigosTriggerEndOverlap OtherActor))

(event EventBeginPlay
  (for _array_element (Actor|GetComponentsByClass "/Script/Engine.ChildActorComponent")
    (bind _asporta_normal (Utilities|Casting|CastToPorta_Normal (Variables|/Script/Engine.ChildActorComponent|GetChildActor _array_element)))
    (Variables|/Game/Blueprints/Portas/Porta_Normal.Porta_Normal_C|SetSalaPai _asporta_normal self)
    (Utilities|Array|Add (Variables|Default|GetPortas) _asporta_normal)))

(event Collision|EventActorBeginOverlap
  (params (OtherActor :type Actor%20Object%20Reference)))

(event EventTick
  (params (DeltaSeconds :type Float%20%28single-precision%29)))

(event EventDestrancarPortas
  (bind _asjogador_bp (Utilities|Casting|CastToJogador_BP (Game|GetPlayerCharacter 0)))
  (Default|EsconderVidaInimigos (Variables|/Game/Blueprints/Jogador/Jogador_BP.Jogador_BP_C|GetJogadorHUD_Ref _asjogador_bp))
  (Class|Sala|AlterarCorSala "(R=0.313997,G=1.000000,B=0.321741,A=1.000000)" (Variables|Default|GetSala)))

(event EventAtualizarVidaInimigos
  (params (jogador :type Jogador%20Object%20Reference))
  (bind _asjogador_bp (Utilities|Casting|CastToJogador_BP jogador))
  (bind _triggerativarinimigos (Variables|Default|GetTriggerAtivarInimigos))
  (bind _jogadorhud_ref (Variables|/Game/Blueprints/Jogador/Jogador_BP.Jogador_BP_C|GetJogadorHUD_Ref _asjogador_bp))
  (Class|Sala|TrancarPortas)
  (Utilities|IsValid _jogadorhud_ref
    (:Is%20Valid
      (bind _output_get (Variables|Default|SetInimigosCopia (Variables|Default|GetInimigos)))
      (Default|SetInimigosAtuais _jogadorhud_ref _output_get)
      (Variables|/Game/UI/Jogo/JogadorHUD.JogadorHUD_C|SetMostrarInimigosBar _jogadorhud_ref true))
    (:Is%20Not%20Valid
      _))
  (EventDispatchers|UnbindallEventsfromOnComponentBeginOverlap _triggerativarinimigos)
  (EventDispatchers|UnbindallEventsfromOnComponentEndOverlap _triggerativarinimigos))

(fn ConstructionScript)