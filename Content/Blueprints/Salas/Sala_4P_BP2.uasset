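; Room Blueprint (Sala) that runs an enemy encounter when the player walks in.
; On BeginPlay it registers itself as parent of its Porta_Normal child-actor doors and collects them.
; If enemies exist, the trigger overlap locks doors, feeds the HUD enemy bar, activates enemies through their AI controllers, then unbinds itself.
; The DestrancarPortas (unlock doors) event hides enemy health on the HUD and recolors the room green.
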(event OnComponentBeginOverlap(TriggerAtivarInimigos)
  (params (OtherActor :type Actor%20Object%20Reference) (OtherComp :type Primitive%20Component%20Object%20Reference) (OtherBodyIndex :type Integer) (bFromSweep :type Boolean) (SweepResult :type Hit%20Result%20Structure%20%28by%20ref%29))
  (bind _asjogador_bp (Utilities|Casting|CastToJogador_BP OtherActor))
  (if (Variables|Default|GetbSalaTemInimigos)
    (Class|Sala|TrancarPortas)
    (bind _output_get (Variables|Default|SetInimigosCopia (Variables|Default|GetInimigos)))
    (Default|SetInimigosAtuais (Variables|/Game/Blueprints/Jogador/Jogador_BP.Jogador_BP_C|GetJogadorHUD_Ref _asjogador_bp) _output_get)
    (Variables|/Game/UI/Jogo/JogadorHUD.JogadorHUD_C|SetMostrarInimigosBar (Variables|/Game/Blueprints/Jogador/Jogador_BP.Jogador_BP_C|GetJogadorHUD_Ref _asjogador_bp) true)
    (for _array_element (Variables|Default|GetInimigos)
      (bind _returnvalue (AI|GetAIController _array_element))
      (Class|InimigosControlador|AtivarInimigo (.AsInimigos%20Controlador (Utilities|Casting|CastToInimigosControlador _returnvalue))))
    (EventDispatchers|UnbindallEventsfromOnComponentBeginOverlap (Variables|Default|GetTriggerAtivarInimigos))))

(event EventBeginPlay
  (for _array_element (Actor|GetComponentsByClass "/Script/Engine.ChildActorComponent")
    (bind _asporta_normal (Utilities|Casting|CastToPorta_Normal (Variables|/Script/Engine.ChildActorComponent|GetChildActor _array_element)))
    (Variables|/Game/Blueprints/Portas/Porta_Normal.Porta_Normal_C|SetSalaPai _asporta_normal self)
    (Utilities|Array|Add (Variables|Default|GetPortas) _asporta_normal)))

(event EventDestrancarPortas
  (bind _asjogador_bp (Utilities|Casting|CastToJogador_BP (Game|GetPlayerCharacter 0)))
  (Default|EsconderVidaInimigos (Variables|/Game/Blueprints/Jogador/Jogador_BP.Jogador_BP_C|GetJogadorHUD_Ref _asjogador_bp))
  (Class|Sala|AlterarCorSala "(R=0.313997,G=1.000000,B=0.321741,A=1.000000)" (Variables|Default|GetSala)))

(fn ConstructionScript)