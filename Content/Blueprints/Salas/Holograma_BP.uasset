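; Room hologram actor that dissolves via a material cut plane and starts player gameplay once fully deactivated.
; The construction script creates HoloGrama's dynamic material; Tick feeds PontoDissolve's world position into its CutPlane parameter and spins Barreiras.
; DesativarHolograma plays a timeline driving the dissolve point, barrier position and spin speed, calling ComeçarJogar on JogadorRef when finished forward.
; AtivarHolograma reverses that timeline to restore the hologram.
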(event Custom|DesativarHolograma
  (bind (_direction _velocidaderotacao _posicao _barreirasposicao) (Timeline|MoverPontoDissolve Play)
    (:Update
      (Transformation|SetWorldLocation (Variables|Default|GetPontoDissolve) _posicao false false)
      (Variables|Default|SetRotateBarreiras _velocidaderotacao)
      (Transformation|SetWorldLocation (Variables|Default|GetBarreiras) _barreirasposicao false false))
    (:Finished
      (switch Utilities|FlowControl|Switch|SwitchonETimelineDirection _direction
        (:Forward
          (Default|ComeçarJogar (Variables|Default|GetJogador_Ref)))))))

(event Custom|AtivarHolograma
  (bind (_direction _velocidaderotacao _posicao _barreirasposicao) (Timeline|MoverPontoDissolve Reverse)
    (:Update
      (Transformation|SetWorldLocation (Variables|Default|GetPontoDissolve) _posicao false false)
      (Variables|Default|SetRotateBarreiras _velocidaderotacao)
      (Transformation|SetWorldLocation (Variables|Default|GetBarreiras) _barreirasposicao false false))
    (:Finished
      (switch Utilities|FlowControl|Switch|SwitchonETimelineDirection _direction
        (:Forward
          (Default|ComeçarJogar (Variables|Default|GetJogador_Ref)))))))

(event EventBeginPlay)

(event EventActorBeginOverlap
  (params (OtherActor :type Actor%20Object%20Reference)))

(event EventTick
  (params (DeltaSeconds :type Float%20%28single-precision%29))
  (Rendering|Material|SetVectorParameterValue (Variables|Default|GetDMI) "CutPlane" (Math|Conversions|ToLinearColor(Vector) (Transformation|GetWorldLocation (Variables|Default|GetPontoDissolve))) :!class /Script/Engine.MaterialInstanceDynamic)
  (Transformation|AddLocalRotation (Variables|Default|GetBarreiras) (Math|Rotator|MakeRotator 0.0 0.0 (* DeltaSeconds (Variables|Default|GetRotateBarreiras))) false false))

(fn ConstructionScript
  (bind _returnvalue (Rendering|Material|CreateDynamicMaterialInstance (Variables|Default|GetHoloGrama) 0 0 :!class /Script/Engine.PrimitiveComponent))
  (bind _output_get (Variables|Default|SetDMI _returnvalue))
  (Rendering|Material|SetVectorParameterValue _output_get "CutPlane" (Math|Conversions|ToLinearColor(Vector) (Transformation|GetWorldLocation (Variables|Default|GetPontoDissolve))) :!class /Script/Engine.MaterialInstanceDynamic))