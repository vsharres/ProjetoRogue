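; Collectible key actor that spins and bobs each tick, using its yaw to drive a sine-based vertical oscillation.
; On BeginPlay it reads the save game, hiding itself and unbinding its trigger if the key is already owned.
; Its trigger offers the player interaction with a custom-depth highlight; pickup hides the key and shows an item popup.
; A second trigger shows the key tutorial once, blocking interaction until then when tutorials are enabled.
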(event OnComponentEndOverlap(TriggerChave)
  (params (OtherActor :type Actor%20Object%20Reference) (OtherComp :type Primitive%20Component%20Object%20Reference) (OtherBodyIndex :type Integer))
  (bind _asjogador_bp (Utilities|Casting|CastToJogador_BP OtherActor))
  (if (not (and (Variables|/Game/Blueprints/Jogador/Jogador_BP.Jogador_BP_C|GetTutorialAtivado _asjogador_bp) (not (Variables|Default|GetTutorialMostrado))))
    (Default|PararInteracao _asjogador_bp)
    (Rendering|SetRenderCustomDepth (Variables|Default|GetChave) false)))

(event OnComponentBeginOverlap(TriggerTutorial)
  (params (OtherActor :type Actor%20Object%20Reference) (OtherComp :type Primitive%20Component%20Object%20Reference) (OtherBodyIndex :type Integer) (bFromSweep :type Boolean) (SweepResult :type Hit%20Result%20Structure%20%28by%20ref%29))
  (bind _asjogador_bp (Utilities|Casting|CastToJogador_BP OtherActor))
  (if (and (Variables|/Game/Blueprints/Jogador/Jogador_BP.Jogador_BP_C|GetTutorialAtivado _asjogador_bp) (not (Variables|Default|GetTutorialMostrado)))
    (Utilities|FlowControl|DoOnce false
      (:Completed
        (Default|MostrarTutorial _asjogador_bp "CHAVE")
        (Utilities|FlowControl|Delay 0.2)
        (Variables|Default|SetTutorialMostrado true)))))

(event OnComponentBeginOverlap(TriggerChave)
  (params (OtherActor :type Actor%20Object%20Reference) (OtherComp :type Primitive%20Component%20Object%20Reference) (OtherBodyIndex :type Integer) (bFromSweep :type Boolean) (SweepResult :type Hit%20Result%20Structure%20%28by%20ref%29))
  (bind _asjogador_bp (Utilities|Casting|CastToJogador_BP OtherActor))
  (if (not (and (Variables|/Game/Blueprints/Jogador/Jogador_BP.Jogador_BP_C|GetTutorialAtivado _asjogador_bp) (not (Variables|Default|GetTutorialMostrado))))
    (Class|InteragirInterface|Interagir(Message) _asjogador_bp "CHAVE" self)
    (Rendering|SetRenderCustomDepth (Variables|Default|GetChave) true)))

(event Custom|PegouChave
  (params (Jogador :type Jogador%20BP%20Object%20Reference))
  (bind _triggerchave (Variables|Default|GetTriggerChave))
  (Rendering|SetVisibility (Variables|Default|GetChave) false false)
  (Class|Jogador|GerarItemPopUp Jogador self)
  (EventDispatchers|UnbindallEventsfromOnComponentBeginOverlap _triggerchave)
  (EventDispatchers|UnbindallEventsfromOnComponentEndOverlap _triggerchave)
  (Default|PararInteracao Jogador))

(event EventTick
  (params (DeltaSeconds :type Float%20%28single-precision%29))
  (CallFunction|RodarChave DeltaSeconds))

(event EventBeginPlay
  (bind _triggerchave (Variables|Default|GetTriggerChave))
  (bind _returnvalue (SaveGame|CreateSaveGameObject "/Script/ProjetoRogue.SalvarJogo"))
  (bind _returnvalue_2 (SaveGame|LoadGamefromSlot (Variables|/Script/ProjetoRogue.SalvarJogo|GetSaveSlot (.AsSalvar%20Jogo (Utilities|Casting|CastToSalvarJogo _returnvalue))) (Variables|/Script/ProjetoRogue.SalvarJogo|GetUserindex (.AsSalvar%20Jogo (Utilities|Casting|CastToSalvarJogo _returnvalue)))))
  (if (Variables|/Script/ProjetoRogue.SalvarJogo|GetbPossuiChave (.AsSalvar%20Jogo (Utilities|Casting|CastToSalvarJogo _returnvalue_2)))
    (Rendering|SetVisibility (Variables|Default|GetChave) false false)
    (EventDispatchers|UnbindallEventsfromOnComponentBeginOverlap _triggerchave)
    (EventDispatchers|UnbindallEventsfromOnComponentEndOverlap _triggerchave)
    (else
      (Variables|Default|SetTutorialMostrado (not (Variables|/Script/ProjetoRogue.SalvarJogo|GetbNovoJogo (.AsSalvar%20Jogo (Utilities|Casting|CastToSalvarJogo _returnvalue_2))))))))

(fn ConstructionScript)

(fn RodarChave
  (params (DeltaTime :type Float%20%28single-precision%29))
  (bind _chave (Variables|Default|GetChave))
  (Transformation|AddWorldRotation _chave (Math|Rotator|MakeRotator 0.0 0.0 (* DeltaTime (LocalVariables|GetVelRotacao))) false false)
  (Transformation|AddWorldOffset _chave (Math|Vector|MakeVector 0.0 0.0 (* (Math|Trig|Sin(Degrees) (.yaw (Transformation|GetWorldRotation _chave))) (LocalVariables|GetVelOscilacao) DeltaTime)) false false))