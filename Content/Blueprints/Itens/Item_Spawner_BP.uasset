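; Item spawner actor that places a random passive or projectile item pickup, which spins and bobs until the player takes it.
; On BeginPlay it hides itself if the save marks the item found, otherwise picks a type from the room generator's seeded stream and sets the matching meshes.
; Trigger overlap shows a one-time tutorial or offers interaction with a custom-depth outline.
; Pickup initializes the item, saves the player and shows a popup.
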(event OnComponentBeginOverlap(TriggerItem)
  (params (OtherActor :type Actor%20Object%20Reference) (OtherComp :type Primitive%20Component%20Object%20Reference) (OtherBodyIndex :type Integer) (bFromSweep :type Boolean) (SweepResult :type Hit%20Result%20Structure%20%28by%20ref%29))
  (bind _asjogador_bp (Utilities|Casting|CastToJogador_BP OtherActor))
  (if (and (Variables|/Game/Blueprints/Jogador/Jogador_BP.Jogador_BP_C|GetTutorialAtivado _asjogador_bp) (not (Variables|Default|GetTutorialMostrado)))
    (Utilities|FlowControl|DoOnce false
      (:Completed
        (switch Utilities|FlowControl|Switch|SwitchonETipoItem (Variables|/Script/ProjetoRogue.Item|GetTipo (Variables|Default|GetItemGerado))
          (:PASSIVO
            (Default|MostrarTutorial _asjogador_bp "ITEMPASSIVO"))
          (:PROJETIL
            (Default|MostrarTutorial _asjogador_bp "ITEMATIVO")))
        (Utilities|FlowControl|Delay 0.2)
        (Variables|Default|SetTutorialMostrado true)))
    (else
      (Class|InteragirInterface|Interagir(Message) _asjogador_bp "ITEM" self)
      (CallFunction|ToggleOutline true))))

(event OnComponentEndOverlap(TriggerItem)
  (params (OtherActor :type Actor%20Object%20Reference) (OtherComp :type Primitive%20Component%20Object%20Reference) (OtherBodyIndex :type Integer))
  (bind _asjogador_bp (Utilities|Casting|CastToJogador_BP OtherActor))
  (if (Variables|Default|GetTutorialMostrado)
    (Default|PararInteracao _asjogador_bp)
    (CallFunction|ToggleOutline false)))

(event Custom|PegouItem
  (params (Jogador :type Jogador%20BP%20Object%20Reference))
  (bind _triggeritem (Variables|Default|GetTriggerItem))
  ;[1 1 1] Inicializar
  (Class|Item|InicializarItem (Variables|Default|GetItemGerado) Jogador)
  (Class|Jogador|SalvarJogador Jogador)
  (Class|Jogador|GerarItemPopUp Jogador self)
  (Rendering|SetVisibility (Variables|Default|GetItem) false true)
  (EventDispatchers|UnbindallEventsfromOnComponentBeginOverlap _triggeritem)
  (EventDispatchers|UnbindallEventsfromOnComponentEndOverlap _triggeritem)
  (Default|PararInteracao Jogador))

(event EventBeginPlay
  (bind _triggeritem (Variables|Default|GetTriggerItem))
  (bind _detalhe_dano (Variables|Default|GetDetalhe_Dano))
  (bind _detalhe_firerate (Variables|Default|GetDetalhe_FireRate))
  (bind _detalhe_precisao (Variables|Default|GetDetalhe_Precisao))
  ;[1 1 1] Inicializar
  (bind _returnvalue (SaveGame|CreateSaveGameObject "/Script/ProjetoRogue.SalvarJogo"))
  (bind _returnvalue_2 (SaveGame|LoadGamefromSlot (Variables|/Script/ProjetoRogue.SalvarJogo|GetSaveSlot (.AsSalvar%20Jogo (Utilities|Casting|CastToSalvarJogo _returnvalue))) (Variables|/Script/ProjetoRogue.SalvarJogo|GetUserindex (.AsSalvar%20Jogo (Utilities|Casting|CastToSalvarJogo _returnvalue)))))
  (if (Variables|/Script/ProjetoRogue.SalvarJogo|GetbItemEncontrado (.AsSalvar%20Jogo (Utilities|Casting|CastToSalvarJogo _returnvalue_2)))
    (Rendering|SetVisibility (Variables|Default|GetItem) false true)
    (EventDispatchers|UnbindallEventsfromOnComponentBeginOverlap _triggeritem)
    (EventDispatchers|UnbindallEventsfromOnComponentEndOverlap _triggeritem)
    (else
      (Variables|Default|SetTipoItem (Utilities|Array|Get(acopy) (Variables|Default|GetPossiveisItens) (Class|KismetMathLibrary|RandomIntegerfromStream (Utilities|Array|LastIndex (Variables|Default|GetPossiveisItens)) (Variables|/Script/ProjetoRogue.SalasGerador|GetStreamGeracao (Class|SalasGerador|GetGeradorSalas)))))
      (Variables|Default|SetTutorialMostrado (not (Variables|/Script/ProjetoRogue.ProtuXGameMode|GetbTutorialAtivado (.AsProtu%20X%20Game%20Mode%20BP (Utilities|Casting|CastToProtuX_GameMode_BP (Game|GetGameMode))))))
      (bind _returnvalue_3 (Class|Item|InstanciarItemBlueprint (Variables|Default|GetTipoItem)))
      (bind _asitem (Utilities|Casting|CastToItem _returnvalue_3))
      (bind _output_get (Variables|Default|SetItemGerado _asitem))
      (switch Utilities|FlowControl|Switch|SwitchonETipoItem (Variables|/Script/ProjetoRogue.Item|GetTipo _output_get)
        (:PASSIVO
          (Rendering|SetVisibility (Variables|Default|GetItemPassivo) true false)
          (Rendering|SetVisibility _detalhe_dano false false)
          (Rendering|SetVisibility _detalhe_firerate false false)
          (Rendering|SetVisibility _detalhe_precisao false false))
        (:PROJETIL
          (Components|StaticMesh|SetStaticMesh _detalhe_dano (Variables|/Script/ProjetoRogue.ItemProjetil|GetDetalheDano (.AsItem%20Projetil (Utilities|Casting|CastToItemProjetil _output_get))))
          (Rendering|Material|SetMaterial _detalhe_dano 0 (Variables|/Script/ProjetoRogue.ItemProjetil|GetDetalheDano_Material (.AsItem%20Projetil (Utilities|Casting|CastToItemProjetil _output_get))))
          (Components|StaticMesh|SetStaticMesh _detalhe_firerate (Variables|/Script/ProjetoRogue.ItemProjetil|GetDetalheFireRate (.AsItem%20Projetil (Utilities|Casting|CastToItemProjetil _output_get))))
          (Rendering|Material|SetMaterial _detalhe_firerate 0 (Variables|/Script/ProjetoRogue.ItemProjetil|GetDetalheFireRate_Material (.AsItem%20Projetil (Utilities|Casting|CastToItemProjetil _output_get))))
          (Components|StaticMesh|SetStaticMesh _detalhe_precisao (Variables|/Script/ProjetoRogue.ItemProjetil|GetDetalhePrecisao (.AsItem%20Projetil (Utilities|Casting|CastToItemProjetil _output_get))))
          (Rendering|Material|SetMaterial _detalhe_precisao 0 (Variables|/Script/ProjetoRogue.ItemProjetil|GetDetalhePrecisao_Material (.AsItem%20Projetil (Utilities|Casting|CastToItemProjetil _output_get))))
          (Rendering|SetVisibility (Variables|Default|GetItemPassivo) false false))))))

(event EventTick
  (params (DeltaSeconds :type Float%20%28single-precision%29))
  (CallFunction|RodarItem DeltaSeconds))

(fn ConstructionScript)

(fn RodarItem
  (params (DeltaTime :type Float%20%28single-precision%29))
  (bind _item (Variables|Default|GetItem))
  (Transformation|AddWorldRotation _item (Math|Rotator|MakeRotator 0.0 0.0 (* DeltaTime (LocalVariables|GetVelRotacao))) false false)
  (Transformation|AddWorldOffset _item (Math|Vector|MakeVector 0.0 0.0 (* (Math|Trig|Sin(Degrees) (.yaw (Transformation|GetWorldRotation _item))) (LocalVariables|GetVelOscilacao) DeltaTime)) false false))

(fn ToggleOutline
  (params (On :type Boolean))
  (Rendering|SetRenderCustomDepth (Variables|Default|GetDetalhe_Dano) On)
  (Rendering|SetRenderCustomDepth (Variables|Default|GetDetalhe_Precisao) On)
  (Rendering|SetRenderCustomDepth (Variables|Default|GetDetalhe_FireRate) On)
  (Rendering|SetRenderCustomDepth (Variables|Default|GetItemPassivo) On))