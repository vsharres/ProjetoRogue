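; Corridor actor that fades its lights in when the player (Jogador_BP) enters TriggerLuz and out when they leave.
; Tick stays off until the first entry, then runs FadeIn every frame without being switched off again.
; FadeIn interpolates point light intensity and the emissive "Intensity" parameter on index-paired Luz_Vidro meshes.
; Speed scales with reverse array index, staggering the fade; the stored player location is unused.
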(event OnComponentBeginOverlap(TriggerLuz)
  (params (OtherActor :type Actor%20Object%20Reference) (OtherComp :type Primitive%20Component%20Object%20Reference) (OtherBodyIndex :type Integer) (bFromSweep :type Boolean) (SweepResult :type Hit%20Result%20Structure%20%28by%20ref%29))
  (bind _asjogador_bp (Utilities|Casting|CastToJogador_BP OtherActor))
  (Variables|Luz|SetFadeLuzes true)
  (Variables|Luz|SetJogadorLoc (Transformation|GetActorLocation _asjogador_bp))
  (Actor|Tick|SetActorTickEnabled true))

(event OnComponentEndOverlap(TriggerLuz)
  (params (OtherActor :type Actor%20Object%20Reference) (OtherComp :type Primitive%20Component%20Object%20Reference) (OtherBodyIndex :type Integer))
  (bind _asjogador_bp (Utilities|Casting|CastToJogador_BP OtherActor))
  (Variables|Luz|SetFadeLuzes false)
  (Variables|Luz|SetJogadorLoc (Transformation|GetActorLocation _asjogador_bp)))

(event EventBeginPlay
  (Variables|Luz|SetLuzes (Actor|GetComponentsByClass "/Script/Engine.PointLightComponent"))
  (Actor|Tick|SetActorTickEnabled false)
  (Variables|Default|SetLuz_Vidros (Actor|GetComponentsbyTag "/Script/Engine.StaticMeshComponent" "Luz_Vidro")))

(event Collision|EventActorBeginOverlap
  (params (OtherActor :type Actor%20Object%20Reference)))

(event EventTick
  (params (DeltaSeconds :type Float%20%28single-precision%29))
  (CallFunction|Fadein))

(fn ConstructionScript)

(fn Fadein
  (bind _luzes (Variables|Luz|GetLuzes))
  (bind _luzes_2 (Variables|Luz|GetLuzes))
  (if (Variables|Luz|GetFadeLuzes)
    (for (_array_element _array_index) _luzes_2
      (Rendering|Components|Light|SetIntensity _array_element (Math|Interpolation|FInterpTo (Variables|/Script/Engine.LightComponentBase|GetIntensity _array_element) 5e+03 (Utilities|Time|GetWorldDeltaSeconds) (* (LocalVariables|GetFadeVel) (Math|Conversions|ToFloat(Integer) (- (Utilities|Array|Length _luzes_2) _array_index)))))
      (bind _returnvalue (Rendering|Material|CreateDynamicMaterialInstance (Utilities|Array|Get(acopy) (Variables|Default|GetLuz_Vidros) _array_index) 0 (Rendering|Material|GetMaterial (Utilities|Array|Get(acopy) (Variables|Default|GetLuz_Vidros) _array_index) 0) :!class /Script/Engine.PrimitiveComponent))
      (bind _returnvalue_2 (Rendering|Material|GetScalarParameterValue _returnvalue "Intensity" :!class /Script/Engine.MaterialInstanceDynamic))
      (Rendering|Material|SetScalarParameterValue _returnvalue "Intensity" (Math|Interpolation|FInterpTo _returnvalue_2 1e+01 (Utilities|Time|GetWorldDeltaSeconds) (* (* (LocalVariables|GetFadeVel) (Math|Conversions|ToFloat(Integer) (- (Utilities|Array|Length _luzes_2) _array_index))) (/ 1e+01 5e+03))) :!class /Script/Engine.MaterialInstanceDynamic))
    (else
      (for (_array_element_2 _array_index_2) _luzes
        (Rendering|Components|Light|SetIntensity _array_element_2 (Math|Interpolation|FInterpTo (Variables|/Script/Engine.LightComponentBase|GetIntensity _array_element_2) 0.0 (Utilities|Time|GetWorldDeltaSeconds) (* (LocalVariables|GetFadeVel) (Math|Conversions|ToFloat(Integer) (- (Utilities|Array|Length _luzes) _array_index_2)))))
        (bind _returnvalue_3 (Rendering|Material|CreateDynamicMaterialInstance (Utilities|Array|Get(acopy) (Variables|Default|GetLuz_Vidros) _array_index_2) 0 (Rendering|Material|GetMaterial (Utilities|Array|Get(acopy) (Variables|Default|GetLuz_Vidros) _array_index_2) 0) :!class /Script/Engine.PrimitiveComponent))
        (bind _returnvalue_4 (Rendering|Material|GetScalarParameterValue _returnvalue_3 "Intensity" :!class /Script/Engine.MaterialInstanceDynamic))
        (Rendering|Material|SetScalarParameterValue _returnvalue_3 "Intensity" (Math|Interpolation|FInterpTo _returnvalue_4 0.0 (Utilities|Time|GetWorldDeltaSeconds) (* (* (LocalVariables|GetFadeVel) (Math|Conversions|ToFloat(Integer) (- (Utilities|Array|Length _luzes) _array_index_2))) (/ 1e+01 5e+03))) :!class /Script/Engine.MaterialInstanceDynamic)))))