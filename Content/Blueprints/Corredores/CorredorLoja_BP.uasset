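; CorredorLoja_BP is a shop corridor actor with a key-type interaction prompt and player-triggered point light fading.
; TriggerLoja starts and stops the Jogador_BP interaction on overlap.
; TriggerLuz sets the fade direction, records the player's location and enables tick on entry.
; FadeLuz interpolates light intensities with speed multiplied (in) or divided (out) by player-to-actor distance, but no graph here calls it, as Event Tick is disabled.
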(event OnComponentBeginOverlap(TriggerLoja)
  (params (OtherActor :type Actor%20Object%20Reference) (OtherComp :type Primitive%20Component%20Object%20Reference) (OtherBodyIndex :type Integer) (bFromSweep :type Boolean) (SweepResult :type Hit%20Result%20Structure%20%28by%20ref%29))
  (bind _asjogador_bp (Utilities|Casting|CastToJogador_BP OtherActor))
  (Class|InteragirInterface|Interagir(Message) _asjogador_bp "CHAVE"))

(event OnComponentBeginOverlap(TriggerLuz)
  (params (OtherActor :type Actor%20Object%20Reference) (OtherComp :type Primitive%20Component%20Object%20Reference) (OtherBodyIndex :type Integer) (bFromSweep :type Boolean) (SweepResult :type Hit%20Result%20Structure%20%28by%20ref%29))
  (bind _asjogador_bp (Utilities|Casting|CastToJogador_BP OtherActor))
  (Variables|Default|SetFadeLuzes true)
  (Variables|Default|SetJogadorLoc (Transformation|GetActorLocation _asjogador_bp))
  (Actor|Tick|SetActorTickEnabled true))

(event OnComponentEndOverlap(TriggerLoja)
  (params (OtherActor :type Actor%20Object%20Reference) (OtherComp :type Primitive%20Component%20Object%20Reference) (OtherBodyIndex :type Integer))
  (bind _asjogador_bp (Utilities|Casting|CastToJogador_BP OtherActor))
  (Class|InteragirInterface|PararInteracao(Message) _asjogador_bp))

(event OnComponentEndOverlap(TriggerLuz)
  (params (OtherActor :type Actor%20Object%20Reference) (OtherComp :type Primitive%20Component%20Object%20Reference) (OtherBodyIndex :type Integer))
  (bind _asjogador_bp (Utilities|Casting|CastToJogador_BP OtherActor))
  (Variables|Default|SetFadeLuzes false)
  (Variables|Default|SetJogadorLoc (Transformation|GetActorLocation _asjogador_bp)))

(event EventBeginPlay
  (Variables|Default|SetLuzes (Actor|GetComponentsByClass "/Script/Engine.PointLightComponent"))
  (Actor|Tick|SetActorTickEnabled false))

(event Collision|EventActorBeginOverlap
  (params (OtherActor :type Actor%20Object%20Reference)))

(event EventTick
  (params (DeltaSeconds :type Float%20%28single-precision%29)))

(fn ConstructionScript)

(fn FadeLuz
  (if (Variables|Default|GetFadeLuzes)
    (for _array_element (Variables|Default|GetLuzes)
      (Rendering|Components|Light|SetIntensity _array_element (Math|Interpolation|FInterpTo (Variables|/Script/Engine.LightComponentBase|GetIntensity _array_element) 5e+03 (Utilities|Time|GetWorldDeltaSeconds) (* (LocalVariables|GetFadeVel) (Math|Vector|VectorLength (- (Transformation|GetActorLocation) (Variables|Default|GetJogadorLoc)))))))
    (else
      (for _array_element_2 (Variables|Default|GetLuzes)
        (Rendering|Components|Light|SetIntensity _array_element_2 (Math|Interpolation|FInterpTo (Variables|/Script/Engine.LightComponentBase|GetIntensity _array_element_2) 0.0 (Utilities|Time|GetWorldDeltaSeconds) (/ (LocalVariables|GetFadeVel) (Math|Conversions|ToFloat(Integer) (Math|Float|Ceil (Math|Vector|VectorLength (- (Transformation|GetActorLocation) (Variables|Default|GetJogadorLoc))))))))))))