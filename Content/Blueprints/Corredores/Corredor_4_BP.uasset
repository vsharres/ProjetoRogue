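; Corridor Blueprint that fades its point lights in when the player (Jogador_BP) enters the TriggerLuz volume and out when they leave.
; BeginPlay caches the lights and disables Tick, which the first player overlap enables permanently.
; Each tick, FadeIn interpolates intensity toward full or zero.
; Interp speed scales FadeVel by actor-to-player distance captured at overlap: multiplied fading in, divided (rounded up) fading out.
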(event OnComponentBeginOverlap(TriggerLuz)
  (params (OtherActor :type Actor%20Object%20Reference) (OtherComp :type Primitive%20Component%20Object%20Reference) (OtherBodyIndex :type Integer) (bFromSweep :type Boolean) (SweepResult :type Hit%20Result%20Structure%20%28by%20ref%29))
  (bind _asjogador_bp (Utilities|Casting|CastToJogador_BP OtherActor))
  (Variables|Luz|SetFadeLuzes true)
  (Variables|Luz|SetJogadorLoc (Transformation|GetActorLocation _asjogador_bp))
  (Actor|Tick|SetActorTickEnabled true))

(event OnComponentEndOverlap(TriggerLuz)
  (params (OtherActor :type Actor%20Object%20Reference) (OtherComp :type Primitive%20Component%20Object%20Reference) (OtherBodyIndex :type Integer))
  (bind _asjogador_bp (Utilities|Casting|CastToJogador_BP OtherActor))
  (Variables|Luz|SetFadeLuzes false)
  (Variables|Luz|SetJogadorLoc (Transformation|GetActorLocation _asjogador_bp)))

(event EventBeginPlay
  (Variables|Luz|SetLuzes (Actor|GetComponentsByClass "/Script/Engine.PointLightComponent"))
  (Actor|Tick|SetActorTickEnabled false))

(event Collision|EventActorBeginOverlap
  (params (OtherActor :type Actor%20Object%20Reference)))

(event EventTick
  (params (DeltaSeconds :type Float%20%28single-precision%29))
  (CallFunction|Fadein))

(fn ConstructionScript)

(fn Fadein
  (if (Variables|Luz|GetFadeLuzes)
    (for _array_element (Variables|Luz|GetLuzes)
      (Rendering|Components|Light|SetIntensity _array_element (Math|Interpolation|FInterpTo (Variables|/Script/Engine.LightComponentBase|GetIntensity _array_element) 5e+03 (Utilities|Time|GetWorldDeltaSeconds) (* (LocalVariables|GetFadeVel) (Math|Vector|VectorLength (- (Transformation|GetActorLocation) (Variables|Luz|GetJogadorLoc)))))))
    (else
      (for _array_element_2 (Variables|Luz|GetLuzes)
        (Rendering|Components|Light|SetIntensity _array_element_2 (Math|Interpolation|FInterpTo (Variables|/Script/Engine.LightComponentBase|GetIntensity _array_element_2) 0.0 (Utilities|Time|GetWorldDeltaSeconds) (/ (LocalVariables|GetFadeVel) (Math|Conversions|ToFloat(Integer) (Math|Float|Ceil (Math|Vector|VectorLength (- (Transformation|GetActorLocation) (Variables|Luz|GetJogadorLoc))))))))))))