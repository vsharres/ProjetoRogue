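; Procedural level generator that, on Inicializar, builds a layout of connected rooms and corridors outward from a starting room.
; A recursive depth-first walk spawns a room and corridor at each unconnected door, using door direction and fixed offsets for placement.
; Room types are random, biased by the parent's door count, until the remaining MaxNumSalas budget forces types with progressively fewer doors.
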(event Custom|Inicializar
  (CallFunction|SetNumeroSalas)
  (Utilities|Array|Add (Variables|Salas|GetSalas) (Variables|Default|GetSala_Inicial))
  (CallFunction|SpawnSalas))

(fn ConstructionScript)

(fn SetNumeroSalas
  (Variables|Salas|SetNumero%20Salas (Utilities|NumeroAleatorio 0 (Variables|Salas|GetMax_Num_Salas))))

(fn SpawnSalas
  (CallFunction|DFSSalas (Utilities|Array|Get(acopy) (Variables|Salas|GetSalas)) (LocalVariables|GetSalas%20Visitadas)))

(fn GetNumPortas
  (params (Tipo :type Sala%20Class%20Reference))
  (if (Utilities|ClassIsChildOf Tipo "/Game/Blueprints/Salas/Sala_1P_BP.Sala_1P_BP_C")
    (LocalVariables|SetNumeroPortas "UMA")
    (elif (Utilities|ClassIsChildOf Tipo "/Game/Blueprints/Salas/Sala_2P_BP.Sala_2P_BP_C")
      (LocalVariables|SetNumeroPortas "UMA")
      (elif (Utilities|ClassIsChildOf Tipo "/Game/Blueprints/Salas/Sala_3P_BP.Sala_3P_BP_C")
        (LocalVariables|SetNumeroPortas "DUAS")
        (else
          (LocalVariables|SetNumeroPortas "TRES")))))
  (return (LocalVariables|GetNumeroPortas)))

(fn GerarTranformSala
  (params (SalaAnterior :type Sala%20Object%20Reference) (DirecaoPorta :type Rotator :default "0, 0, 0"))
  (bind _returnvalue (Transformation|GetActorLocation SalaAnterior))
  (bind _returnvalue_2 (Math|Rotator|GetRotationXVector DirecaoPorta))
  (bind _offset_sala (Variables|Default|GetOffset_Sala))
  (return (Math|Transform|MakeTransform (Math|Vector|MakeVector (+ (* (.x _returnvalue_2) _offset_sala) (.x _returnvalue)) (+ (* _offset_sala (.y _returnvalue_2)) (.y _returnvalue)) 0.0) (Math|Vector|RotatorfromAxisandAngle "0, 0,1.000000" (+ (* (.x _returnvalue_2) 1.8e+02) (* (.y _returnvalue_2) -9e+01))) (LocalVariables|GetEscala%20Padrao))))

(fn GerarTransformCorredor
  (params (Sala :type Sala%20Object%20Reference) (DirecaoPorta :type Rotator :default "0, 0, 0"))
  (bind _returnvalue (Transformation|GetActorLocation Sala))
  (bind _returnvalue_2 (Math|Rotator|GetRotationXVector DirecaoPorta))
  (bind _offset_corredor (Variables|Default|GetOffset_Corredor))
  (return (Math|Transform|MakeTransform (Math|Vector|MakeVector (+ (* (.x _returnvalue_2) _offset_corredor) (.x _returnvalue)) (+ (* _offset_corredor (.y _returnvalue_2)) (.y _returnvalue)) (.z _returnvalue)) (Math|Vector|RotatorfromAxisandAngle "0, 0,1.000000" (+ (* (.x _returnvalue_2) 1.8e+02) (* (.y _returnvalue_2) 9e+01))) (LocalVariables|GetEscalaPadrao))))

(fn DFSSalas
  (params (Sala%20Atual :type Sala%20Object%20Reference) (Salas%20Visitadas :type Array%20of%20Sala%20Object%20References))
  (bind _salas_conectadas (Variables|/Script/ProjetoRogue.Sala|GetSalas_Conectadas Sala%20Atual))
  (bind _numero_portas (Variables|/Script/ProjetoRogue.Sala|GetNumero_Portas Sala%20Atual))
  (bind _returnvalue (Math|Conversions|ToInteger(Byte) _numero_portas))
  (Utilities|Array|Add Salas%20Visitadas Sala%20Atual)
  (Variables|/Script/ProjetoRogue.Sala|SetbVisited Sala%20Atual true)
  (if (== 0 _returnvalue)
    _
    (else
      (for _index (range (+ (Utilities|Array|Length _salas_conectadas) 1) _returnvalue)
        (bind _direaoporta (CallFunction|GetDirecaoPorta _index (Transformation|GetActorRotation Sala%20Atual)))
        (CallFunction|GerarSala Sala%20Atual _direaoporta))))
  (for _array_element _salas_conectadas
    (if (not (Variables|/Script/ProjetoRogue.Sala|GetbVisited _array_element))
      (CallFunction|DFSSalas _array_element Salas%20Visitadas))))

(fn GerarSala
  (params (SalaParente :type Sala%20Object%20Reference) (DirecaoPorta :type Rotator :default "0, 0, 0"))
  (bind _salas (Variables|Salas|GetSalas))
  (bind _output_get (LocalVariables|SetParente SalaParente))
  (bind _transformsala (CallFunction|GerarTranformSala _output_get DirecaoPorta))
  (bind _tipo_de_sala (CallFunction|SelecionarTipoSala (LocalVariables|GetParente)))
  (bind _returnvalue (Game|SpawnActorfromClass _tipo_de_sala _transformsala true 0))
  (bind _output_get_2 (LocalVariables|SetSalaGerada _returnvalue))
  (Utilities|Array|Add (Variables|/Script/ProjetoRogue.Sala|GetSalas_Conectadas (LocalVariables|GetParente)) _output_get_2)
  (Utilities|Array|Add (Variables|/Script/ProjetoRogue.Sala|GetSalas_Conectadas _output_get_2) (LocalVariables|GetParente))
  (bind _return_transform (CallFunction|GerarTransformCorredor (LocalVariables|GetParente) DirecaoPorta))
  (Game|SpawnActorfromClass "/Game/Blueprints/Salas/Corredor_BP.Corredor_BP_C" _return_transform true 0)
  (Utilities|Array|Resize _salas (+ (Utilities|Array|Length _salas) (Math|Conversions|ToInteger(Byte) (Variables|/Script/ProjetoRogue.Sala|GetNumero_Portas (LocalVariables|GetSalaGerada)))))
  (Utilities|Array|SetArrayElem (Variables|Salas|GetSalas) (+ (Utilities|Array|FindItem _salas (LocalVariables|GetParente)) 1) (LocalVariables|GetSalaGerada)))

(fn GetDirecaoPorta
  (params (IndicePorta :type Integer :default 0) (DirecaoSala :type Rotator :default "0, 0, 0"))
  (bind (_pitch _yaw _roll) (Class|KismetMathLibrary|BreakRot DirecaoSala))
  (bind (_pitch_2 _yaw_2 _roll_2) (Class|KismetMathLibrary|BreakRot DirecaoSala))
  (bind (_pitch_3 _yaw_3 _roll_3) (Class|KismetMathLibrary|BreakRot DirecaoSala))
  (switch int IndicePorta
    (:1
      (LocalVariables|SetPortaRotator DirecaoSala))
    (:2
      (LocalVariables|SetPortaRotator (Class|KismetMathLibrary|MakeRot _pitch (+ _yaw 1.8e+02) _roll)))
    (:3
      (LocalVariables|SetPortaRotator (Class|KismetMathLibrary|MakeRot _pitch_2 (+ _yaw_2 9e+01) _roll_2)))
    (:4
      (LocalVariables|SetPortaRotator (Class|KismetMathLibrary|MakeRot _pitch_3 (+ _yaw_3 -9e+01) _roll_3))))
  (return (LocalVariables|GetPortaRotator)))

(fn SelecionarTipoSala
  (params (Sala%20Parente :type Sala%20Object%20Reference))
  (bind _tipos_salas_disponiveis (Variables|Salas|GetTipos_Salas_Disponiveis))
  (bind _salas (Variables|Salas|GetSalas))
  (bind _max_num_salas (Variables|Salas|GetMax_Num_Salas))
  (bind _returnvalue (Utilities|Array|Length _salas))
  (bind _returnvalue_2 (- _max_num_salas _returnvalue))
  (if (<= _returnvalue_2 1)
    (LocalVariables|SetRetornarTipo "/Game/Blueprints/Salas/Sala_1P_BP.Sala_1P_BP_C")
    (elif (<= _returnvalue_2 2)
      (LocalVariables|SetRetornarTipo "/Game/Blueprints/Salas/Sala_2P_BP.Sala_2P_BP_C")
      (elif (<= _returnvalue_2 3)
        (LocalVariables|SetRetornarTipo "/Game/Blueprints/Salas/Sala_3P_BP.Sala_3P_BP_C")
        (elif (<= _returnvalue_2 4)
          (LocalVariables|SetRetornarTipo "/Game/Blueprints/Salas/Sala_4P_BP.Sala_4P_BP_C")
          (else
            (if (> (Variables|/Script/ProjetoRogue.Sala|GetNumero_Portas Sala%20Parente) 1)
              (LocalVariables|SetIndice 0)
              (else
                (LocalVariables|SetIndice 3)))
            (bind _output_get (LocalVariables|SetRetornarTipo (Utilities|Array|Get(acopy) _tipos_salas_disponiveis (Utilities|NumeroAleatorio (LocalVariables|GetIndice) (Utilities|Array|LastIndex _tipos_salas_disponiveis))))))))))
  (return _output_get))