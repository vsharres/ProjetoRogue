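; Drone enemy Blueprint that damages the player on contact and flashes when hit.
; Overlaps on ColisorDano pass damage from Stats to the Jogador's ReceberDano, gated by a short cooldown that refills on Tick, and flag the drone as attacking.
; FlashDano writes the current game time into a material parameter for the hit flash and sets the player as the AI blackboard's target.
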(event OnComponentBeginOverlap(ColisorDano)
  (params (OtherActor :type Actor%20Object%20Reference) (OtherComp :type Primitive%20Component%20Object%20Reference) (OtherBodyIndex :type Integer) (bFromSweep :type Boolean) (SweepResult :type Hit%20Result%20Structure%20%28by%20ref%29))
  (bind _asjogador (Utilities|Casting|CastToJogador OtherActor))
  (if (Math|Float|NearlyEqual(Float) (Variables|Default|GetDanoCooldown) 3.0 0.01)
    (Variables|Default|SetbEstaAtacando true)
    (Class|Jogador|ReceberDano _asjogador (.dano (Variables|Default|GetStats)) 0 SweepResult)
    (Variables|Default|SetDanoCooldown 0.0)))

(event EventFlashDano
  (bind _mesh (Variables|Character|GetMesh))
  (bind _returnvalue (Rendering|Material|CreateDynamicMaterialInstance _mesh 0 (Rendering|Material|GetMaterial _mesh 0) :!class /Script/Engine.PrimitiveComponent))
  (Rendering|Material|SetScalarParameterValue _returnvalue "Time_Hit" (Utilities|Time|GetGameTimeinSeconds) :!class /Script/Engine.MaterialInstanceDynamic)
  (AI|Components|Blackboard|SetValueasObject (AI|GetBlackboard (.AsAIController (Utilities|Casting|CastToAIController (Pawn|GetController)))) (Variables|Default|GetJogador) (Game|GetPlayerCharacter 0)))

(event EventBeginPlay)

(event Collision|EventActorBeginOverlap
  (params (OtherActor :type Actor%20Object%20Reference)))

(event EventTick
  (params (DeltaSeconds :type Float%20%28single-precision%29))
  (if (< (Variables|Default|GetDanoCooldown) 3.0)
    (Variables|Default|SetDanoCooldown (+ (Variables|Default|GetDanoCooldown) DeltaSeconds))
    (else
      (Variables|Default|SetDanoCooldown 3.0))))

(fn ConstructionScript)