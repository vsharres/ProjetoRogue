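; Prototype "Spreeder" enemy that extends parent shooting, throttling it by its fire rate stat.
; Damage flashes timestamp dynamic material parameters and set player zero as the AI blackboard target.
; Death runs once: it disables collision and the AI controller, starts a timed material effect, spawns a pickup, plays a sound, then destroys the actor after the material's death duration.
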(event EventAtirar
  (Utilities|FlowControl|DoOnce false :!label _label
    (:Completed
      (|CallParentFunction)
      (Utilities|FlowControl|Delay (/ 1.0 (.firerate (Variables|Default|GetStats))))
      (goto _label Reset))))

(event EventBeginPlay)

(event Collision|EventActorBeginOverlap
  (params (OtherActor :type Actor%20Object%20Reference)))

(event EventTick
  (params (DeltaSeconds :type Float%20%28single-precision%29)))

(event EventFlashDano
  (for _array_element (Rendering|Material|GetMaterials (Variables|Character|GetMesh))
    (bind _returnvalue (Rendering|Material|CreateDynamicMaterialInstance _array_element :!class /Script/Engine.KismetMaterialLibrary))
    (Rendering|Material|SetScalarParameterValue _returnvalue "Time_Hit" (Utilities|Time|GetGameTimeinSeconds) :!class /Script/Engine.MaterialInstanceDynamic)
    (AI|Components|Blackboard|SetValueasObject (AI|GetBlackboard (.AsAIController (Utilities|Casting|CastToAIController (Pawn|GetController)))) (Variables|Default|GetJogador) (Game|GetPlayerCharacter 0))))

(event EventInimigoMorreu
  (bind _mesh (Variables|Character|GetMesh))
  (Utilities|FlowControl|DoOnce false
    (:Completed
      (Collision|SetCollisionEnabled (Variables|Default|GetCapsuleComponent) "NoCollision")
      (Class|InimigosControlador|DesativarInimigo (.AsProto%20Controlador (Utilities|Casting|CastToProto_Controlador (Pawn|GetController))))
      (Variables|Default|SetbEstaMorrendo true)
      (for (_ _array_index) (Rendering|Material|GetMaterials _mesh)
        (bind _returnvalue (Rendering|Material|CreateDynamicMaterialInstance _mesh _array_index 0 :!class /Script/Engine.PrimitiveComponent))
        (Rendering|Material|SetScalarParameterValue _returnvalue "Time_Death" (Utilities|Time|GetGameTimeinSeconds) :!class /Script/Engine.MaterialInstanceDynamic)
        (bind _returnvalue_2 (Rendering|Material|GetScalarParameterValue _returnvalue "Duration_Death" :!class /Script/Engine.MaterialInstanceDynamic))
        (Variables|Default|SetTempoEspera _returnvalue_2))
      (Class|Inimigo|SpawnPickUp)
      (Audio|PlaySoundatLocation "/Game/Sons/Efeitos/Boss/Damage_Obliterate02_Cue.Damage_Obliterate02_Cue" (Transformation|GetActorLocation))
      (Utilities|FlowControl|Delay (Variables|Default|GetTempoEspera))
      (Actor|DestroyActor))))

(fn ConstructionScript)