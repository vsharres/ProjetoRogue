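; Boss enemy character that punches the player with left and right hand colliders and handles its hit flash and death.
; Fist overlaps deal damage and horizontal knockback only during that hand's attack, gated by a Tick-recharged cooldown.
; FlashDano timestamps dynamic materials for the hit effect and sets the player in the AI blackboard.
; Death disables capsule collision and AI, timestamps the death effect, spawns a pickup, then destroys the actor after the material's duration.
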(event OnComponentBeginOverlap(Colisor_L)
  (params (OtherActor :type Actor%20Object%20Reference) (OtherComp :type Primitive%20Component%20Object%20Reference) (OtherBodyIndex :type Integer) (bFromSweep :type Boolean) (SweepResult :type Hit%20Result%20Structure%20%28by%20ref%29))
  (bind _asjogador_bp (Utilities|Casting|CastToJogador_BP OtherActor))
  (if (Math|Float|NearlyEqual(Float) (Variables|Default|GetDanoCooldown) 1.0 0.01)
    (if (and (Variables|Default|GetbEstaAtacando) (Variables|Default|GetAtacandoComEsquerda))
      (Class|Jogador|ReceberDano _asjogador_bp (.dano (Variables|Default|GetStats)) 0 SweepResult)
      (Character|LaunchCharacter _asjogador_bp (* (Math|Vector|MakeVector (.x (Math|Rotator|GetRotationXVector (Math|Rotator|FindLookatRotation (Transformation|GetActorLocation) (Transformation|GetActorLocation _asjogador_bp)))) (.y (Math|Rotator|GetRotationXVector (Math|Rotator|FindLookatRotation (Transformation|GetActorLocation) (Transformation|GetActorLocation _asjogador_bp)))) 0.0) (Variables|Default|GetForcaSoco)) false false)
      (Variables|Default|SetDanoCooldown 0.0))))

(event OnComponentBeginOverlap(Colisor_R)
  (params (OtherActor :type Actor%20Object%20Reference) (OtherComp :type Primitive%20Component%20Object%20Reference) (OtherBodyIndex :type Integer) (bFromSweep :type Boolean) (SweepResult :type Hit%20Result%20Structure%20%28by%20ref%29))
  (bind _asjogador_bp (Utilities|Casting|CastToJogador_BP OtherActor))
  (if (Math|Float|NearlyEqual(Float) (Variables|Default|GetDanoCooldown) 1.0 0.01)
    (if (and (Variables|Default|GetbEstaAtacando) (Variables|Default|GetAtacandoComDireita))
      (Class|Jogador|ReceberDano _asjogador_bp (.dano (Variables|Default|GetStats)) 0 SweepResult)
      (Character|LaunchCharacter _asjogador_bp (* (Math|Vector|MakeVector (.x (Math|Rotator|GetRotationXVector (Math|Rotator|FindLookatRotation (Transformation|GetActorLocation) (Transformation|GetActorLocation _asjogador_bp)))) (.y (Math|Rotator|GetRotationXVector (Math|Rotator|FindLookatRotation (Transformation|GetActorLocation) (Transformation|GetActorLocation _asjogador_bp)))) 0.0) (Variables|Default|GetForcaSoco)) false false)
      (Variables|Default|SetDanoCooldown 0.0))))

(event EventBeginPlay)

(event Collision|EventActorBeginOverlap
  (params (OtherActor :type Actor%20Object%20Reference)))

(event EventTick
  (params (DeltaSeconds :type Float%20%28single-precision%29))
  (if (< (Variables|Default|GetDanoCooldown) 1.0)
    (Variables|Default|SetDanoCooldown (+ (Variables|Default|GetDanoCooldown) DeltaSeconds))
    (else
      (Variables|Default|SetDanoCooldown 1.0))))

(event EventFlashDano
  (for (_ _array_index) (Rendering|Material|GetMaterials (Variables|Character|GetMesh))
    (bind _returnvalue (Rendering|Material|CreateDynamicMaterialInstance (Variables|Character|GetMesh) _array_index 0 :!class /Script/Engine.PrimitiveComponent))
    (Rendering|Material|SetScalarParameterValue _returnvalue "Time_Hit" (Utilities|Time|GetGameTimeinSeconds) :!class /Script/Engine.MaterialInstanceDynamic)
    (AI|Components|Blackboard|SetValueasObject (AI|GetBlackboard (.AsAIController (Utilities|Casting|CastToAIController (Pawn|GetController)))) (Variables|Default|GetJogador) (Game|GetPlayerCharacter 0))))

(event EventInimigoMorreu
  (bind _mesh (Variables|Character|GetMesh))
  (Utilities|FlowControl|DoOnce false
    (:Completed
      (Collision|SetCollisionEnabled (Variables|Default|GetCapsuleComponent) "NoCollision")
      (Class|InimigosControlador|DesativarInimigo (.AsBoss%20Controlador%20BP (Utilities|Casting|CastToBossControlador_BP (Pawn|GetController))))
      (Variables|Default|SetbEstaMorrendo true)
      (for (_ _array_index) (Rendering|Material|GetMaterials _mesh)
        (bind _returnvalue (Rendering|Material|CreateDynamicMaterialInstance _mesh _array_index 0 :!class /Script/Engine.PrimitiveComponent))
        (Rendering|Material|SetScalarParameterValue _returnvalue "Time_Death" (Utilities|Time|GetGameTimeinSeconds) :!class /Script/Engine.MaterialInstanceDynamic)
        (bind _returnvalue_2 (Rendering|Material|GetScalarParameterValue _returnvalue "Duration_Death" :!class /Script/Engine.MaterialInstanceDynamic))
        (Variables|Default|SetTempoEspera _returnvalue_2))
      (Class|Inimigo|SpawnPickUp)
      (Utilities|FlowControl|Delay (Variables|Default|GetTempoEspera))
      (Actor|DestroyActor))))

(fn ConstructionScript)