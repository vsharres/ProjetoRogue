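; HoloLog is an interactable hologram log that holds a text entry chosen from a data table.
; On BeginPlay it picks a random row by numeric name using the room generator's seeded stream and stores that row's text.
; An overlap component registers it with the player's interaction system and toggles custom depth on its mesh while the player is in range.
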(event OnComponentBeginOverlap(AtivarHoloLog)
  (params (OtherActor :type Actor%20Object%20Reference) (OtherComp :type Primitive%20Component%20Object%20Reference) (OtherBodyIndex :type Integer) (bFromSweep :type Boolean) (SweepResult :type Hit%20Result%20Structure%20%28by%20ref%29))
  (bind _asjogador_bp (Utilities|Casting|CastToJogador_BP OtherActor))
  (Default|Interagir _asjogador_bp "NENHUMA" self)
  (Rendering|SetRenderCustomDepth (Variables|Default|GetMesh) true))

(event OnComponentEndOverlap(AtivarHoloLog)
  (params (OtherActor :type Actor%20Object%20Reference) (OtherComp :type Primitive%20Component%20Object%20Reference) (OtherBodyIndex :type Integer))
  (bind _asjogador_bp (Utilities|Casting|CastToJogador_BP OtherActor))
  (Default|PararInteracao _asjogador_bp)
  (Rendering|SetRenderCustomDepth (Variables|Default|GetMesh) false))

(event EventBeginPlay
  (bind _returnvalue (Class|SalasGerador|GetGeradorSalas))
  (bind _outrownames (DataTable|GetDataTableRowNames "/Game/Blueprints/HoloLog/Teste_DataTable.Teste_DataTable"))
  (bind _output_get (Variables|Default|SetNumLogs (Utilities|Array|Length _outrownames)))
  (Variables|Default|SetSeed (Variables|/Script/ProjetoRogue.SalasGerador|GetSeed _returnvalue))
  (bind _returnvalue_2 (Utilities|GetDataTableRow "/Game/Blueprints/HoloLog/Teste_DataTable.Teste_DataTable" (Utilities|String|StringToName (Utilities|String|ToString(Integer) (Math|Random|RandomIntegerinRangefromStream 1 _output_get (Variables|/Script/ProjetoRogue.SalasGerador|GetStreamGeracao _returnvalue)))))
    (:then
      (Variables|Default|SetTextoLog (Utilities|Text|ToText(String) (Utilities|Struct|BreakHoloLogTable _returnvalue_2))))))

(event EventActorBeginOverlap
  (params (OtherActor :type Actor%20Object%20Reference)))

(event EventTick
  (params (DeltaSeconds :type Float%20%28single-precision%29)))

(fn ConstructionScript)