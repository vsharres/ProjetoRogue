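; Boss room, a specialised room that spawns a random or selected boss and controls its encounter and exit elevator.
; SpawnInimigos extends the parent spawn, adding a boss from PossiveisBoss unless the save marks it defeated.
; BeginPlay links child-actor boss doors to the room and raises the elevator if already defeated.
; A one-shot trigger activates the first enemy's AI and boss HUD bar; DestrancarPortas hides it and raises the elevator.
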(event OnComponentBeginOverlap(TriggerBoss)
  (params (OtherActor :type Actor%20Object%20Reference) (OtherComp :type Primitive%20Component%20Object%20Reference) (OtherBodyIndex :type Integer) (bFromSweep :type Boolean) (SweepResult :type Hit%20Result%20Structure%20%28by%20ref%29))
  (bind _asjogador_bp (Utilities|Casting|CastToJogador_BP OtherActor))
  (CallFunction|AtivarBoss _asjogador_bp)
  (EventDispatchers|UnbindallEventsfromOnComponentBeginOverlap (Variables|Default|GetTriggerBoss)))

(event Custom|AtivarBoss
  (params (Jogador :type Jogador%20BP%20Object%20Reference))
  (bind _jogadorhud_ref (Variables|/Game/Blueprints/Jogador/Jogador_BP.Jogador_BP_C|GetJogadorHUD_Ref Jogador))
  (bind _output_get (Variables|Default|SetInimigosCopia (Variables|Default|GetInimigos)))
  (Default|SetInimigosAtuais _jogadorhud_ref _output_get)
  (Default|NomearBoss _jogadorhud_ref)
  (Variables|/Game/UI/Jogo/JogadorHUD.JogadorHUD_C|SetMostrarInimigosBar _jogadorhud_ref true)
  (bind _returnvalue (AI|GetAIController (Utilities|Array|Get(acopy) (Variables|Default|GetInimigos))))
  (Class|InimigosControlador|AtivarInimigo (.AsInimigos%20Controlador (Utilities|Casting|CastToInimigosControlador _returnvalue))))

(event EventDestrancarPortas
  (bind _asjogador_bp (Utilities|Casting|CastToJogador_BP (Game|GetPlayerCharacter 0)))
  (Utilities|IsValid (Variables|/Game/Blueprints/Jogador/Jogador_BP.Jogador_BP_C|GetJogadorHUD_Ref _asjogador_bp)
    (:Is%20Valid
      (Default|EsconderVidaInimigos (Variables|/Game/Blueprints/Jogador/Jogador_BP.Jogador_BP_C|GetJogadorHUD_Ref _asjogador_bp))
      (Default|SubirElevador (Variables|Default|GetElevador)))))

(event EventBeginPlay
  (for _array_element (Actor|GetComponentsByClass "/Script/Engine.ChildActorComponent")
    (bind _asporta_boss (Utilities|Casting|CastToPorta_Boss (Variables|/Script/Engine.ChildActorComponent|GetChildActor _array_element)))
    (Variables|/Script/ProjetoRogue.Porta|SetSalaPai _asporta_boss self)
    (Utilities|Array|Add (Variables|Default|GetPortas) _asporta_boss)
    (bind _output_get (Variables|Default|SetElevador (.AsElevador%20Boss%20BP (Utilities|Casting|CastToElevador_Boss_BP (Variables|/Script/Engine.ChildActorComponent|GetChildActor (Variables|Default|GetElevadorComp))))))
    (if (Variables|/Script/ProjetoRogue.SalvarJogo|GetbBossDerrotado (Variables|Default|GetSaveGame))
      (Default|SubirElevador _output_get))))

(event Collision|EventActorBeginOverlap
  (params (OtherActor :type Actor%20Object%20Reference)))

(event EventTick
  (params (DeltaSeconds :type Float%20%28single-precision%29)))

(fn ConstructionScript
  (|CallParentFunction))

(fn SpawnInimigos
  (bind _boss_spawner (Variables|Default|GetBoss_Spawner))
  (bind _returnvalue (SaveGame|CreateSaveGameObject "/Script/ProjetoRogue.SalvarJogo"))
  (bind _returnvalue_2 (SaveGame|LoadGamefromSlot (Variables|/Script/ProjetoRogue.SalvarJogo|GetSaveSlot (.AsSalvar%20Jogo (Utilities|Casting|CastToSalvarJogo _returnvalue))) (Variables|/Script/ProjetoRogue.SalvarJogo|GetUserindex (.AsSalvar%20Jogo (Utilities|Casting|CastToSalvarJogo _returnvalue)))))
  (bind _output_get (Variables|Default|SetSaveGame (.AsSalvar%20Jogo (Utilities|Casting|CastToSalvarJogo _returnvalue_2))))
  (if (and (Variables|Boss|GetbTemBoss) (not (Variables|/Script/ProjetoRogue.SalvarJogo|GetbBossDerrotado _output_get)))
    (bind _stream (|CallParentFunction))
    (bind _returnvalue_3 (Class|Sala|GetTipoInimigo (Variables|Boss|GetPossiveisBoss)))
    (bind _returnvalue_4 (Game|SpawnActorfromClass _returnvalue_3 (Math|Transform|MakeTransform (Transformation|GetWorldLocation _boss_spawner) (Transformation|GetWorldRotation _boss_spawner) "1.000000,1.000000,1.000000") "AdjustIfPossibleButDontSpawnIfColliding" 0 0))
    (Utilities|IsValid _returnvalue_4
      (:Is%20Valid
        (bind _output_get_2 (Variables|Boss|SetBoss _returnvalue_4))
        (Pawn|SpawnDefaultController _output_get_2)
        (Utilities|Array|Add (Variables|Default|GetInimigos) _output_get_2)
        (Variables|/Script/ProjetoRogue.Inimigo|SetSalaPai _output_get_2 self)
        (return _stream))
      (:Is%20Not%20Valid
        (bind _stream_2 (|CallParentFunction))
        (return _stream_2)))
    (else
      (bind _stream_3 (|CallParentFunction))
      (return _stream_3))))