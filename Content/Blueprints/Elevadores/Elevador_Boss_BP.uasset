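; Boss elevator that rises, dissolves its holographic tube, then later takes the player back down and ends play via TerminarJogar.
; SubirElevador drives a height timeline, then the hologram timeline, which moves a dissolve point feeding the tube material's CutPlane and disables collision.
; Player overlap disables input and, after a delay, reverses the hologram while easing the player to the tube's centre, then reverses the lift.
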(event OnComponentBeginOverlap(TriggerElevador)
  (params (OtherActor :type Actor%20Object%20Reference) (OtherComp :type Primitive%20Component%20Object%20Reference) (OtherBodyIndex :type Integer) (bFromSweep :type Boolean) (SweepResult :type Hit%20Result%20Structure%20%28by%20ref%29))
  (bind _asjogador_bp (Utilities|Casting|CastToJogador_BP OtherActor))
  (bind _output_get (Variables|Default|SetJogador _asjogador_bp))
  (Input|DisableInput _output_get (Game|GetPlayerController 0))
  (Utilities|FlowControl|Delay 1.0)
  (CallFunction|AtivarHolograma))

(event Custom|DesativarHolograma
  (bind _returnvalue (Utilities|Time|GetWorldDeltaSeconds))
  (bind _pontodissolver (Variables|Default|GetPontoDissolver))
  (bind _jogador (Variables|Default|GetJogador))
  (bind _elevador_tubo (Variables|Default|GetElevador_Tubo))
  (bind _returnvalue_2 (Transformation|GetActorLocation _jogador))
  (bind _returnvalue_3 (Transformation|GetWorldLocation _elevador_tubo))
  (bind _relativelocation (Variables|/Script/Engine.SceneComponent|GetRelativeLocation _pontodissolver))
  (bind _returnvalue_4 (Math|Interpolation|VInterpTo _returnvalue_2 _returnvalue_3 _returnvalue 5.0))
  (bind (_direction _pontodissolverposz) (Timeline|DesativarHolo Play)
    (:Update
      (Transformation|SetRelativeLocation _pontodissolver (Math|Vector|MakeVector (.x _relativelocation) (.y _relativelocation) _pontodissolverposz) false false)
      (switch Utilities|FlowControl|Switch|SwitchonETimelineDirection _direction
        (:Backward
          (Utilities|IsValid _jogador
            (:Is%20Valid
              (Transformation|SetActorLocation _jogador (Math|Vector|MakeVector (.x _returnvalue_4) (.y _returnvalue_4) (.Z (Math|Vector|BreakVector _returnvalue_2))) false false))))))
    (:Finished
      (switch Utilities|FlowControl|Switch|SwitchonETimelineDirection _direction
        (:Forward
          (Collision|SetCollisionEnabled (Variables|Default|GetElevador_Tubo) "NoCollision"))
        (:Backward
          (CallFunction|DescerElevador))))))

(event Custom|AtivarHolograma
  (bind _returnvalue (Utilities|Time|GetWorldDeltaSeconds))
  (bind _pontodissolver (Variables|Default|GetPontoDissolver))
  (bind _jogador (Variables|Default|GetJogador))
  (bind _elevador_tubo (Variables|Default|GetElevador_Tubo))
  (bind _returnvalue_2 (Transformation|GetActorLocation _jogador))
  (bind _returnvalue_3 (Transformation|GetWorldLocation _elevador_tubo))
  (bind _relativelocation (Variables|/Script/Engine.SceneComponent|GetRelativeLocation _pontodissolver))
  (bind _returnvalue_4 (Math|Interpolation|VInterpTo _returnvalue_2 _returnvalue_3 _returnvalue 5.0))
  (bind (_direction _pontodissolverposz) (Timeline|DesativarHolo Reverse)
    (:Update
      (Transformation|SetRelativeLocation _pontodissolver (Math|Vector|MakeVector (.x _relativelocation) (.y _relativelocation) _pontodissolverposz) false false)
      (switch Utilities|FlowControl|Switch|SwitchonETimelineDirection _direction
        (:Backward
          (Utilities|IsValid _jogador
            (:Is%20Valid
              (Transformation|SetActorLocation _jogador (Math|Vector|MakeVector (.x _returnvalue_4) (.y _returnvalue_4) (.Z (Math|Vector|BreakVector _returnvalue_2))) false false))))))
    (:Finished
      (switch Utilities|FlowControl|Switch|SwitchonETimelineDirection _direction
        (:Forward
          (Collision|SetCollisionEnabled (Variables|Default|GetElevador_Tubo) "NoCollision"))
        (:Backward
          (CallFunction|DescerElevador))))))

(event Custom|SubirElevador
  (bind _returnvalue (Transformation|GetActorLocation))
  (bind (_direction _posicaoz) (Timeline|Subir Play)
    (:Update
      (Transformation|SetActorLocation (Math|Vector|MakeVector (.x _returnvalue) (.y _returnvalue) _posicaoz) false false))
    (:Finished
      (switch Utilities|FlowControl|Switch|SwitchonETimelineDirection _direction
        (:Forward
          (CallFunction|DesativarHolograma))))))

(event Custom|DescerElevador
  (bind _returnvalue (Transformation|GetActorLocation))
  (Default|TerminarJogar (Variables|Default|GetJogador))
  (bind (_direction _posicaoz) (Timeline|Subir Reverse)
    (:Update
      (Transformation|SetActorLocation (Math|Vector|MakeVector (.x _returnvalue) (.y _returnvalue) _posicaoz) false false))
    (:Finished
      (switch Utilities|FlowControl|Switch|SwitchonETimelineDirection _direction
        (:Forward
          (CallFunction|DesativarHolograma))))))

(event EventBeginPlay)

(event EventActorBeginOverlap
  (params (OtherActor :type Actor%20Object%20Reference)))

(event EventTick
  (params (DeltaSeconds :type Float%20%28single-precision%29))
  (Rendering|Material|SetVectorParameterValue (Variables|Default|GetDMI) "CutPlane" (Math|Conversions|ToLinearColor(Vector) (Transformation|GetWorldLocation (Variables|Default|GetPontoDissolver))) :!class /Script/Engine.MaterialInstanceDynamic))

(fn ConstructionScript
  (bind _returnvalue (Rendering|Material|CreateDynamicMaterialInstance (Variables|Default|GetElevador_Tubo) 0 0 :!class /Script/Engine.PrimitiveComponent))
  (bind _output_get (Variables|Default|SetDMI _returnvalue))
  (Rendering|Material|SetVectorParameterValue _output_get "CutPlane" (Math|Conversions|ToLinearColor(Vector) (Transformation|GetWorldLocation (Variables|Default|GetPontoDissolver))) :!class /Script/Engine.MaterialInstanceDynamic))