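; Next-level elevator Blueprint that lowers itself at BeginPlay, dissolves its hologram tube and then hands control to the player.
; A Descer timeline drives the actor's height, and when it finishes the DesativarHolo timeline moves the PontoDissolver point vertically before calling ComeçarJogar on Jogador_BP.
; Tick feeds that point's world position into the CutPlane parameter of a dynamic material on ElevadorTubo, created in the construction script.
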(event Custom|DesativarHolograma
  (bind _pontodissolver (Variables|Default|GetPontoDissolver))
  (bind _relativelocation (Variables|/Script/Engine.SceneComponent|GetRelativeLocation _pontodissolver))
  (bind _pontodissolverposz (Timeline|DesativarHolo Play)
    (:Update
      (Transformation|SetRelativeLocation _pontodissolver (Math|Vector|MakeVector (.x _relativelocation) (.y _relativelocation) _pontodissolverposz) false false))
    (:Finished
      (Default|ComeçarJogar (Variables|Default|GetJogador)))))

(event Custom|DescerElevador
  (bind _returnvalue (Transformation|GetActorLocation))
  (bind _posicaoz (Timeline|Descer Play)
    (:Update
      (Transformation|SetActorLocation (Math|Vector|MakeVector (.x _returnvalue) (.y _returnvalue) _posicaoz) false false))
    (:Finished
      (CallFunction|DesativarHolograma))))

(event EventBeginPlay
  (Variables|Default|SetJogador (.AsJogador%20BP (Utilities|Casting|CastToJogador_BP (Game|Player|GetPlayerPawn 0))))
  (CallFunction|DescerElevador))

(event Collision|EventActorBeginOverlap
  (params (OtherActor :type Actor%20Object%20Reference)))

(event EventTick
  (params (DeltaSeconds :type Float%20%28single-precision%29))
  (Rendering|Material|SetVectorParameterValue (Variables|Default|GetDMI) "CutPlane" (Math|Conversions|ToLinearColor(Vector) (Transformation|GetWorldLocation (Variables|Default|GetPontoDissolver))) :!class /Script/Engine.MaterialInstanceDynamic))

(fn ConstructionScript
  (bind _returnvalue (Rendering|Material|CreateDynamicMaterialInstance (Variables|Default|GetElevador_Tubo) 0 0 :!class /Script/Engine.PrimitiveComponent))
  (bind _output_get (Variables|Default|SetDMI _returnvalue))
  (Rendering|Material|SetVectorParameterValue _output_get "CutPlane" (Math|Conversions|ToLinearColor(Vector) (Transformation|GetWorldLocation (Variables|Default|GetPontoDissolver))) :!class /Script/Engine.MaterialInstanceDynamic))