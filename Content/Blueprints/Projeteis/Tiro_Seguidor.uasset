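; Homing projectile Blueprint that locks onto a pawn entering its target-detection collider, ColisorAlvos.
; While Ativo is true, the first overlapping pawn other than the Instigator has its root component set as CompMovimentacao's homing target.
; A DoOnce keeps that first target locked until the Atingiu (hit) event resets it for a new acquisition.
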(event OnComponentBeginOverlap(ColisorAlvos)
  (params (OtherActor :type Actor%20Object%20Reference) (OtherComp :type Primitive%20Component%20Object%20Reference) (OtherBodyIndex :type Integer) (bFromSweep :type Boolean) (SweepResult :type Hit%20Result%20Structure%20%28by%20ref%29))
  (bind _aspawn (Utilities|Casting|CastToPawn OtherActor))
  (if (and (!= _aspawn (Variables|Default|GetInstigator)) (Variables|Default|GetbAtivo))
    (Utilities|FlowControl|DoOnce false
      (:Completed
        (Variables|/Script/Engine.ProjectileMovementComponent|SetHomingTargetComponent (Variables|Default|GetCompMovimentacao) (VehicleSound|GetRootComponent _aspawn))))))

(event EventAtingiu
  (Utilities|FlowControl|DoOnce false) ; enters at Reset
)

(event EventBeginPlay)

(event Collision|EventActorBeginOverlap
  (params (OtherActor :type Actor%20Object%20Reference)))

(event EventTick
  (params (DeltaSeconds :type Float%20%28single-precision%29)))

(fn ConstructionScript)