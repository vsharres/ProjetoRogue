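; Piercing projectile (Tiro_Penetrante) that damages enemies or players it overlaps and passes through them.
; On overlap, targets implementing DanoInterface are cast to Inimigo or Jogador and receive ReceberDano with the damage from its Stats.
; A hit counter lets it continue until MaxInimigos is reached, then a further damaging hit destroys it.
; Overlapping anything without the interface, or any blocking hit, destroys it immediately.
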(event OnComponentHit(CompCollisao)
  (params (OtherActor :type Actor%20Object%20Reference) (OtherComp :type Primitive%20Component%20Object%20Reference) (NormalImpulse :type Vector :default "0, 0, 0") (Hit :type Hit%20Result%20Structure%20%28by%20ref%29))
  (Actor|DestroyActor))

(event OnComponentBeginOverlap(CompCollisao)
  (params (OtherActor :type Actor%20Object%20Reference) (OtherComp :type Primitive%20Component%20Object%20Reference) (OtherBodyIndex :type Integer) (bFromSweep :type Boolean) (SweepResult :type Hit%20Result%20Structure%20%28by%20ref%29))
  (bind _stats (Variables|Default|GetStats))
  (if (Utilities|DoesObjectImplementInterface OtherActor "/Script/ProjetoRogue.DanoInterface")
    (bind _asinimigo (Utilities|Casting|CastToInimigo OtherActor)
      (:then
        (Class|Inimigo|ReceberDano _asinimigo (.dano _stats)))
      (:CastFailed
        (bind _asjogador (Utilities|Casting|CastToJogador OtherActor))
        (Class|Jogador|ReceberDano _asjogador (.dano _stats))))
    (if (< (Variables|Default|GetNumInimigos) (Variables|Default|GetMaxInimigos))
      (Variables|Default|SetNumInimigos (+ (Variables|Default|GetNumInimigos) 1))
      (else
        (Actor|DestroyActor)))
    (else
      (Actor|DestroyActor))))

(event EventBeginPlay)

(event Collision|EventActorBeginOverlap
  (params (OtherActor :type Actor%20Object%20Reference)))

(event EventTick
  (params (DeltaSeconds :type Float%20%28single-precision%29)))

(fn ConstructionScript)