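; Normal door Blueprint meant to slide open along local Y once its parent room (SalaPai) has no enemies.
; AbrirPorta offsets the mesh by speed times delta time up to a maximum displacement, re-calling PortaAberta, which closes the Gate that feeds it.
; The enemy check that opens and enters that Gate is unconnected and Tick is empty, so nothing here drives the movement.
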(event Custom|PortaAberta
  (Utilities|FlowControl|Gate true) ; enters at Close
)

(event EventBeginPlay)

(event EventTick
  (params (DeltaSeconds :type Float%20%28single-precision%29)))

(fn ConstructionScript)

(fn AbrirPorta?
  (params (Delta%20Seconds :type Float%20%28single-precision%29))
  (bind _velocidadeporta (Variables|Default|GetVelocidadePorta))
  (bind _returnvalue (* Delta%20Seconds _velocidadeporta))
  (if (Variables|Default|GetAbrirPorta)
    (if (< (Variables|Default|GetDelocamento) (Variables|Default|GetDeslocamentoMax))
      (Variables|Default|SetDelocamento (+ (Variables|Default|GetDelocamento) _returnvalue))
      (CallFunction|PortaAberta)
      (Transformation|AddLocalOffset (Variables|Default|GetPortaMesh) (Math|Vector|MakeVector 0.0 _returnvalue 0.0) false)))
  (return))