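; Lockable two-panel sliding door that opens when the player (Jogador) enters its Box trigger and closes when they leave.
; DestrancarPorta and TrancarPorta toggle the lock and swap a PortaMesh glow material; the lock is checked only on overlap begin.
; Every Tick, MoverPortas uses FInterpTo to slide both panels apart along relative Y or back to zero, driven by AbrirPorta.
; FecharPorta is set but never read here.
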(event OnComponentBeginOverlap(Box)
  (params (OtherActor :type Actor%20Object%20Reference) (OtherComp :type Primitive%20Component%20Object%20Reference) (OtherBodyIndex :type Integer) (bFromSweep :type Boolean) (SweepResult :type Hit%20Result%20Structure%20%28by%20ref%29))
  (Utilities|Casting|CastToJogador OtherActor)
  (if (not (Variables|Default|GetbPortaTrancada))
    (Variables|Default|SetbAbrirPorta true)
    (Variables|Default|SetbFecharPorta false)))

(event OnComponentEndOverlap(Box)
  (params (OtherActor :type Actor%20Object%20Reference) (OtherComp :type Primitive%20Component%20Object%20Reference) (OtherBodyIndex :type Integer))
  (Utilities|Casting|CastToJogador OtherActor)
  (Variables|Default|SetbAbrirPorta false)
  (Variables|Default|SetbFecharPorta true))

(event EventBeginPlay)

(event EventTick
  (params (DeltaSeconds :type Float%20%28single-precision%29))
  (CallFunction|MoverPortas DeltaSeconds))

(event EventTrancarPorta
  (Variables|Default|SetbPortaTrancada true)
  (Rendering|Material|SetMaterial (Variables|Default|GetPortaMesh) 1 "/Game/Materiais/Glow/Glow_Chao_Boss_Inst.Glow_Chao_Boss_Inst"))

(event EventDestrancarPorta
  (Variables|Default|SetbPortaTrancada false)
  (Rendering|Material|SetMaterial (Variables|Default|GetPortaMesh) 1 "/Game/Materiais/Glow/Glow_Parede_Inst.Glow_Parede_Inst"))

(fn ConstructionScript)

(fn MoverPortas
  (params (Delta%20Seconds :type Float%20%28single-precision%29))
  (bind _velocidadeporta (Variables|Default|GetVelocidadePorta))
  (bind _porta_1 (Variables|Default|GetPorta_1))
  (bind _porta_2 (Variables|Default|GetPorta_2))
  (bind _velocidadeporta_2 (Variables|Default|GetVelocidadePorta))
  (bind _porta_1_2 (Variables|Default|GetPorta_1))
  (bind _porta_2_2 (Variables|Default|GetPorta_2))
  (bind _relativelocation (Variables|/Script/Engine.SceneComponent|GetRelativeLocation _porta_1))
  (bind _relativelocation_2 (Variables|/Script/Engine.SceneComponent|GetRelativeLocation _porta_2))
  (bind _relativelocation_3 (Variables|/Script/Engine.SceneComponent|GetRelativeLocation _porta_1_2))
  (bind _relativelocation_4 (Variables|/Script/Engine.SceneComponent|GetRelativeLocation _porta_2_2))
  (if (Variables|Default|GetbAbrirPorta)
    (Transformation|SetRelativeLocation (Variables|Default|GetPorta_1) (Math|Vector|MakeVector (.x _relativelocation_3) (Math|Interpolation|FInterpTo (.y _relativelocation_3) (Variables|Default|GetDeslocamento) Delta%20Seconds _velocidadeporta_2) (.z _relativelocation_3)) false false)
    (Transformation|SetRelativeLocation (Variables|Default|GetPorta_2) (Math|Vector|MakeVector (.x _relativelocation_4) (Math|Interpolation|FInterpTo (.y _relativelocation_4) (* (Variables|Default|GetDeslocamento) -1.0) Delta%20Seconds _velocidadeporta_2) (.z _relativelocation_4)) false false)
    (else
      (Transformation|SetRelativeLocation (Variables|Default|GetPorta_1) (Math|Vector|MakeVector (.x _relativelocation) (Math|Interpolation|FInterpTo (.y _relativelocation) 0.0 Delta%20Seconds _velocidadeporta) (.z _relativelocation)) false false)
      (Transformation|SetRelativeLocation (Variables|Default|GetPorta_2) (Math|Vector|MakeVector (.x _relativelocation_2) (Math|Interpolation|FInterpTo (.y _relativelocation_2) 0.0 Delta%20Seconds _velocidadeporta) (.z _relativelocation_2)) false false)))
  (return))