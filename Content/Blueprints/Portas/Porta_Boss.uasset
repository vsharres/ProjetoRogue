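; Boss door that slides open for a player carrying the key and, without one, stays closed with red lights or shows a one-time tutorial.
; Trigger overlaps set open/close flags and reveal the key mesh; Tick eases both panels and the key with FInterpTo.
; When the key holder leaves the trigger, it closes and locks if the parent room has enemies.
; Lock/unlock events swap the glow material and recolor all point lights.
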(event OnComponentBeginOverlap(TriggerPorta)
  (params (OtherActor :type Actor%20Object%20Reference) (OtherComp :type Primitive%20Component%20Object%20Reference) (OtherBodyIndex :type Integer) (bFromSweep :type Boolean) (SweepResult :type Hit%20Result%20Structure%20%28by%20ref%29))
  (bind _asjogador_bp (Utilities|Casting|CastToJogador_BP OtherActor))
  (if (Math|Boolean|ANDBoolean (Variables|/Game/Blueprints/Jogador/Jogador_BP.Jogador_BP_C|GetTutorialAtivado _asjogador_bp) (not (Variables|/Script/ProjetoRogue.Jogador|GetbPossuiChave _asjogador_bp)) (not (Variables|Default|GetTutorialMostrado)))
    (Utilities|FlowControl|DoOnce false
      (:Completed
        (Default|MostrarTutorial _asjogador_bp "PORTACHEFE")
        (Variables|Default|SetTutorialMostrado true)))
    (elif (not (Variables|Default|GetbPortaTrancada))
      (if (Variables|/Script/ProjetoRogue.Jogador|GetbPossuiChave _asjogador_bp)
        (Class|Porta|DestrancarPorta)
        (Utilities|FlowControl|Sequence
          (:then_0
            (Utilities|FlowControl|DoOnce false
              (:Completed
                (Rendering|Material|SetMaterial (Variables|Default|GetPortaMesh) 1 "/Game/Materiais/Glow/Glow_Parede_Chave_Inst.Glow_Parede_Chave_Inst")
                (Rendering|SetVisibility (Variables|Default|GetChave) true false)
                (Utilities|FlowControl|Delay 2.0))))
          (:then_1
            (Variables|Default|SetbAbrirPorta true)
            (Variables|Default|SetbFecharPorta false)))
        (else
          (Variables|Default|SetbAbrirPorta false)
          (Variables|Default|SetbFecharPorta true)
          (Rendering|Material|SetMaterial (Variables|Default|GetPortaMesh) 1 "/Game/Materiais/Glow/Glow_Parede_Boss_Inst.Glow_Parede_Boss_Inst")
          (CallFunction|ToggleLuzes true))))))

(event OnComponentEndOverlap(TriggerPorta)
  (params (OtherActor :type Actor%20Object%20Reference) (OtherComp :type Primitive%20Component%20Object%20Reference) (OtherBodyIndex :type Integer))
  (bind _asjogador (Utilities|Casting|CastToJogador OtherActor))
  (if (Variables|/Script/ProjetoRogue.Jogador|GetbPossuiChave _asjogador)
    (Variables|Default|SetbAbrirPorta false)
    (Variables|Default|SetbFecharPorta true)
    (if (Variables|/Script/ProjetoRogue.Sala|GetbSalaTemInimigos (Variables|Default|GetSalaPai))
      (Class|Porta|TrancarPorta))))

(event EventBeginPlay)

(event Collision|EventActorBeginOverlap
  (params (OtherActor :type Actor%20Object%20Reference)))

(event EventTick
  (params (DeltaSeconds :type Float%20%28single-precision%29))
  (CallFunction|MoverPorta DeltaSeconds)
  (CallFunction|MoverChave DeltaSeconds))

(event EventTrancarPorta
  (Variables|Default|SetbPortaTrancada true)
  (Rendering|Material|SetMaterial (Variables|Default|GetPortaMesh) 1 "/Game/Materiais/Glow/Glow_Parede_Boss_Inst.Glow_Parede_Boss_Inst")
  (CallFunction|ToggleLuzes true))

(event EventDestrancarPorta
  (Variables|Default|SetbPortaTrancada false)
  (Rendering|Material|SetMaterial (Variables|Default|GetPortaMesh) 1 "/Game/Materiais/Glow/Glow_Parede_Chave_Inst.Glow_Parede_Chave_Inst")
  (CallFunction|ToggleLuzes false))

(fn ConstructionScript)

(fn MoverPorta
  (params (DeltaSeconds :type Float%20%28single-precision%29))
  (bind _velocidadeporta (Variables|Default|GetVelocidadePorta))
  (bind _porta_1 (Variables|Default|GetPorta_1))
  (bind _porta_2 (Variables|Default|GetPorta_2))
  (bind _velocidadeporta_2 (Variables|Default|GetVelocidadePorta))
  (bind _porta_1_2 (Variables|Default|GetPorta_1))
  (bind _porta_2_2 (Variables|Default|GetPorta_2))
  (bind _relativelocation (Variables|/Script/Engine.SceneComponent|GetRelativeLocation _porta_1))
  (bind _relativelocation_2 (Variables|/Script/Engine.SceneComponent|GetRelativeLocation _porta_2))
  (bind _relativelocation_3 (Variables|/Script/Engine.SceneComponent|GetRelativeLocation _porta_1_2))
  (bind _relativelocation_4 (Variables|/Script/Engine.SceneComponent|GetRelativeLocation _porta_2_2))
  (if (Variables|Default|GetbAbrirPorta)
    (Transformation|SetRelativeLocation (Variables|Default|GetPorta_1) (Math|Vector|MakeVector (.x _relativelocation_3) (Math|Interpolation|FInterpTo (.y _relativelocation_3) (Variables|Default|GetDelocamento) DeltaSeconds _velocidadeporta_2) (.z _relativelocation_3)) false false)
    (Transformation|SetRelativeLocation (Variables|Default|GetPorta_2) (Math|Vector|MakeVector (.x _relativelocation_4) (Math|Interpolation|FInterpTo (.y _relativelocation_4) (* (Variables|Default|GetDelocamento) -1.0) DeltaSeconds _velocidadeporta_2) (.z _relativelocation_4)) false false)
    (else
      (Transformation|SetRelativeLocation (Variables|Default|GetPorta_1) (Math|Vector|MakeVector (.x _relativelocation) (Math|Interpolation|FInterpTo (.y _relativelocation) 0.0 DeltaSeconds _velocidadeporta) (.z _relativelocation)) false false)
      (Transformation|SetRelativeLocation (Variables|Default|GetPorta_2) (Math|Vector|MakeVector (.x _relativelocation_2) (Math|Interpolation|FInterpTo (.y _relativelocation_2) 0.0 DeltaSeconds _velocidadeporta) (.z _relativelocation_2)) false false))))

(fn ToggleLuzes
  (params (Vermelho :type Boolean))
  (bind _returnvalue (Actor|GetComponentsByClass "/Script/Engine.PointLightComponent"))
  (if Vermelho
    (for _array_element _returnvalue
      (Rendering|Components|Light|SetLightColor _array_element "(R=0.776471,G=0.388236,B=0.392647,A=1.000000)" true))
    (else
      (for _array_element_2 _returnvalue
        (Rendering|Components|Light|SetLightColor _array_element_2 "(R=1.000000,G=0.931132,B=0.861076,A=1.000000)" true)))))

(fn MoverChave
  (params (DeltaTime :type Float%20%28single-precision%29))
  (bind _chave (Variables|Default|GetChave))
  (bind _relativelocation (Variables|/Script/Engine.SceneComponent|GetRelativeLocation _chave))
  (if (Rendering|IsVisible _chave)
    (Transformation|SetRelativeLocation _chave (Math|Vector|MakeVector (Math|Interpolation|FInterpTo (.x _relativelocation) -46.0 DeltaTime (LocalVariables|GetVelChave)) (.y _relativelocation) (.z _relativelocation)) false false)))